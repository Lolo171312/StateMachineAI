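; BP_Char is a golem character with a Paper2D sprite and a widget health bar.
; It caches the WB_HealthBar widget on BeginPlay and exposes events to set the bar's percent and swap the sprite.
; Each Tick, it switches the widget between two mirrored rotations and offsets based on actor yaw.
; An unconnected branch that would turn the widget toward a camera actor never runs.
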(event EventSetHealthBar
  (params (NewPercent :type Float%20%28single-precision%29))
  (Utilities|IsValid (Variables|Default|GetHealthBarWidget)
    (:Is%20Valid
      (Class|HealthBarWidget|SetHealthBarPercent (Variables|Default|GetHealthBarWidget) NewPercent))))

(event EventBeginPlay
  (bind _aswb_health_bar (Utilities|Casting|CastToWB_HealthBar (UserInterface|GetWidget (Variables|Default|GetWidget))))
  (Variables|Default|SetHealthBarWidget _aswb_health_bar))

(event EventSetGolemSpriteTexture
  (params (NewGolemTexture :type Paper%20Sprite%20Object%20Reference))
  (Rendering|Components|Sprite|SetSprite (Variables|Default|GetPaperSprite) NewGolemTexture))

(event EventTick
  (params (DeltaSeconds :type Float%20%28single-precision%29))
  (bind _widget (Variables|Default|GetWidget))
  (if (> (Math|Float|Absolute(Float) (.yaw (Transformation|GetActorRotation))) 9e+01)
    (Transformation|SetRelativeRotation _widget "0.000000,270.000000,0.000000" false false)
    (Transformation|SetRelativeLocation _widget "25.000000,-300.000000,250.000000" false false)
    (else
      (Transformation|SetRelativeRotation _widget "0.000000,90.000000,0.000000" false false)
      (Transformation|SetRelativeLocation _widget "25.000000,300.000000,250.000000" false false))))

(fn ConstructionScript)